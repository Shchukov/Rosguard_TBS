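; BP_Pawn is a player-controlled camera pawn with panning, stepped yaw rotation and spring arm zoom.
; Input axes move a desired location along the actor's forward and right vectors and adjust a clamped desired zoom, while left and right action presses offset a desired rotation.
; Tick smoothly interpolates the actor's location, rotation and spring arm length toward these targets, which start from the initial values at BeginPlay.
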(event `self.ReceiveBeginPlay`
  (set `self.LocationDesired` (`self.K2_GetActorLocation`))
  (set `self.ZoomDesired` (`SpringArmComponent.TargetArmLength` (`self.SpringArm`)))
  (set `self.RotationDesired` (`self.K2_GetActorRotation`)))

(event `self.ReceiveTick`
  (params (DeltaSeconds :type "Float (single-precision)"))
  (bind _springarm (`self.SpringArm`))
  (set `SpringArmComponent.TargetArmLength` (`KismetMathLibrary.FInterpTo` (`SpringArmComponent.TargetArmLength` _springarm) (`self.ZoomDesired`) DeltaSeconds (`self.Zoom_InterpSpeed`)) _springarm)
  (`self.K2_SetActorLocation` (`KismetMathLibrary.VInterpTo` (`self.K2_GetActorLocation`) (`self.LocationDesired`) DeltaSeconds (`self.Location_InterpSpeed`)))
  (`self.K2_SetActorRotation` (`KismetMathLibrary.RInterpTo` (`self.K2_GetActorRotation`) (`self.RotationDesired`) DeltaSeconds (`self.Rotation_InterpSpeed`))))

(event `InputAxis|Zoom`
  (params (AxisValue :type "Float (single-precision)"))
  (set `self.ZoomDesired` (`KismetMathLibrary.FClamp` (+ (* AxisValue (`self.Zoom_Speed`)) (`self.ZoomDesired`)) (`self.Zoom_Min`) (`self.Zoom_Max`))))

(event `InputAxis|Forward`
  (params (AxisValue :type "Float (single-precision)"))
  (set `self.LocationDesired` (+ (`self.LocationDesired`) (* (* AxisValue (`self.Location_Speed`)) (`self.GetActorForwardVector`)))))

(event `InputAxis|Right`
  (params (AxisValue :type "Float (single-precision)"))
  (set `self.LocationDesired` (+ (`self.LocationDesired`) (* (* AxisValue (`self.Location_Speed`)) (`self.GetActorRightVector`)))))

(event `InputAction|RotationRight`
  (params (Key :type "Key Structure"))
  (:`Pressed`
    (set `self.RotationDesired` (`KismetMathLibrary.ComposeRotators` (`self.RotationDesired`) (`KismetMathLibrary.MakeRotator` 0.0 0.0 (- 0.0 (`self.Rotation_Speed`)))))))

(event `InputAction|RotationLeft`
  (params (Key :type "Key Structure"))
  (:`Pressed`
    (set `self.RotationDesired` (`KismetMathLibrary.ComposeRotators` (`self.RotationDesired`) (`KismetMathLibrary.MakeRotator` 0.0 0.0 (`self.Rotation_Speed`))))))

(fn `UserConstructionScript`)